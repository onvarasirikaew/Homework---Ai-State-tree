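; BP_Enemy is an enemy Blueprint that tracks health and carries an overhead widget.
; On BeginPlay it casts its Widget component's user widget to WBP_EnemyOverhead, stores it and passes itself in as EnemyRef.
; AnyDamage subtracts incoming damage from Health and checks for zero or below, but that death branch is empty.
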(event `self.ReceiveBeginPlay`
  (bind _aswbp_enemy_overhead (cast `/Game/WBP_EnemyOverhead` (`WidgetComponent.GetUserWidgetObject` (`self.Widget`))))
  (set `self.OverheadWidget` _aswbp_enemy_overhead)
  (set `/Game/WBP_EnemyOverhead.EnemyRef` self _aswbp_enemy_overhead))

(event `self.ReceiveAnyDamage`
  (params (Damage :type "Float (single-precision)") (DamageType :type "DamageType Object Reference") (InstigatedBy :type "Controller Object Reference") (DamageCauser :type "Actor Object Reference"))
  (bind _output_get (set `self.Health` (- (`self.Health`) Damage)))
  (if (<= _output_get 0.0)
    _))

(fn `UserConstructionScript`)